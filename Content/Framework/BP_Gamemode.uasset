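; BP_Gamemode is the game mode that spawns RTS player controllers at player starts when a match begins.
; On HandleStartingNewPlayer it registers each controller and reads the expected player count and solo flag from BP_GameInstance.
; Solo games spawn the first controller immediately at start "0".
; Otherwise it waits until every expected player has joined, pauses briefly, then restarts each controller at the start named by its join index.
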(event EventBeginPlay)

(event EventTick
  (params (DeltaSeconds :type Float%20%28single-precision%29)))

(event EventHandleStartingNewPlayer
  (params (NewPlayer :type Player%20Controller%20Object%20Reference))
  (bind _asbp_rtsplayer_controller (Utilities|Casting|CastToBP_RTSPlayerController NewPlayer))
  (Utilities|Array|Add (Variables|Default|GetAll_ConnectedControllers) _asbp_rtsplayer_controller)
  (bind _asbp_game_instance (Utilities|Casting|CastToBP_GameInstance (Game|GetGameInstance)))
  (Variables|Default|SetNum_ExpectedPlayers (Variables|/Game/Framework/BP_GameInstance.BP_GameInstance_C|GetNumber%20Of%20Connected%20Players _asbp_game_instance))
  (if (Variables|/Game/Framework/BP_GameInstance.BP_GameInstance_C|GetIsSoloGame _asbp_game_instance)
    (Variables|Default|SetNum_ExpectedPlayers 1)
    (Class|GameModeBase|RestartPlayeratPlayerStart (Utilities|Array|Get(acopy) (Variables|Default|GetAll_ConnectedControllers)) (Class|GameModeBase|FindPlayerStart 0 "0"))
    (elif (== (Variables|Default|GetNum_ExpectedPlayers) (Utilities|Array|Length (Variables|Default|GetAll_ConnectedControllers)))
      (Utilities|FlowControl|Delay 0.5)
      (for (_array_element _array_index) (Variables|Default|GetAll_ConnectedControllers)
        (Class|GameModeBase|RestartPlayeratPlayerStart _array_element (Class|GameModeBase|FindPlayerStart _array_element (Utilities|String|ToString(Integer) _array_index)))))))

(fn ConstructionScript)