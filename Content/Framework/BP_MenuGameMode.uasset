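; Game mode for the RTS menus that manages players in the multiplayer lobby.
; On the Lobby Menu Map, each new player's menu controller is tracked, then told to create its lobby menu and run initial setup.
; UpdateLobby rebuilds the profile list from connected controllers and pushes names or the selected level to each one.
; Logout removes the controller and refreshes the name list for remaining players.
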(event Custom|UpdateLobby
  (params (PlayerNames :type Boolean) (LevelSelection :type Boolean))
  ;[1 1 1] Update Lobby, can be expanded to include maps, factions etc..
  (if PlayerNames
    (Utilities|Array|Clear (Variables|Default|GetAll_PlayerProfiles))
    (for _array_element (Variables|Default|GetAll_ConnectedPlayers)
      (Utilities|Array|Add (Variables|Default|GetAll_PlayerProfiles) (Variables|/Game/Framework/BP_RTSMenuController.BP_RTSMenuController_C|GetPlayerProfileInfo _array_element))))
  (for _array_element_2 (Variables|Default|GetAll_ConnectedPlayers)
    (if PlayerNames
      (Default|UpdatePlayerNames _array_element_2 (Variables|Default|GetAll_PlayerProfiles)))
    (if LevelSelection
      (Default|UpdateLevelSelection _array_element_2 (Variables|Default|GetSelectedLevelName)))))

(event EventOnLogout
  (params (ExitingController :type Controller%20Object%20Reference))
  ;[1 1 1] Update player lobby
  (bind _asbp_rtsmenu_controller (Utilities|Casting|CastToBP_RTSMenuController ExitingController))
  (Utilities|Array|RemoveItem (Variables|Default|GetAll_ConnectedPlayers) _asbp_rtsmenu_controller)
  (CallFunction|UpdateLobby true false))

(event EventHandleStartingNewPlayer
  (params (NewPlayer :type Player%20Controller%20Object%20Reference))
  ;[1 1 1] Add new player to playercontroller
  (bind _returnvalue (Game|GetCurrentLevelName true))
  (switch string _returnvalue
    (:LobbyMenu_Map
      (bind _asbp_rtsmenu_controller (Utilities|Casting|CastToBP_RTSMenuController NewPlayer))
      (Utilities|Array|Add (Variables|Default|GetAll_ConnectedPlayers) _asbp_rtsmenu_controller)
      (Default|CreateLobbyMenu _asbp_rtsmenu_controller)
      (Default|InitialSetup _asbp_rtsmenu_controller))))

(fn ConstructionScript)