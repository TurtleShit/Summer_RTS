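; Menu game mode that manages the multiplayer lobby's player list and keeps connected menu controllers in sync.
; New players on the lobby map are registered and get their lobby menu created; logouts remove them and refresh the lobby.
; UpdateLobby rebuilds the profile array in controller order, copies profiles to player states, then pushes names or level selection to every controller.
; Its faction, team and color flags are currently unused.
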(event Custom|UpdateLobby
  (params (PlayerNames :type Boolean) (LevelSelection :type Boolean) (Faction :type Boolean) (Team :type Boolean) (Color :type Boolean))
  ;[1 1 1] Update Lobby, can be expanded to include maps, factions etc..
  (Utilities|Array|Clear (Variables|Default|GetAll_PlayerProfiles))
  (for (_array_element _array_index) (Variables|Default|GetAll_ConnectedPlayers)
    (Utilities|Array|SetArrayElem (Variables|Default|GetAll_PlayerProfiles) _array_index (Variables|/Game/Framework/Menu/BP_RTSMenuController.BP_RTSMenuController_C|GetPlayerProfileInfo _array_element) true) ; Ensure that we always have the right index to the players
    (bind _asbp_rts_player_state (Utilities|Casting|CastToBP_RTS_PlayerState (Variables|/Script/Engine.Controller|GetPlayerState _array_element)))
    (Variables|/Game/Framework/Gameplay/BP_RTS_PlayerState.BP_RTS_PlayerState_C|SetS_PlayerProfile _asbp_rts_player_state (Variables|/Game/Framework/Menu/BP_RTSMenuController.BP_RTSMenuController_C|GetPlayerProfileInfo _array_element)))
  (for _array_element_2 (Variables|Default|GetAll_ConnectedPlayers)
    (if PlayerNames
      (Default|UpdatePlayerNames _array_element_2 (Variables|Default|GetAll_PlayerProfiles)))
    (if LevelSelection
      (Default|UpdateLevelSelection _array_element_2 (Variables|Default|GetSelectedLevelName)))))

(event EventOnLogout
  (params (ExitingController :type Controller%20Object%20Reference))
  ;[1 1 1] Handle Player Logout
  (bind _asbp_rtsmenu_controller (Utilities|Casting|CastToBP_RTSMenuController ExitingController))
  (Utilities|Array|RemoveItem (Variables|Default|GetAll_ConnectedPlayers) _asbp_rtsmenu_controller)
  (CallFunction|UpdateLobby true false true true true))

(event EventPostLogin
  (params (NewPlayer :type Player%20Controller%20Object%20Reference)))

(event EventHandleStartingNewPlayer
  (params (NewPlayer :type Player%20Controller%20Object%20Reference))
  ;[1 1 1] Add new player to playercontroller
  (bind _returnvalue (Game|GetCurrentLevelName true))
  (switch string _returnvalue ; Execute rest of code IF we are in lobby map
    (:LobbyMenu_Map
      (bind _asbp_rtsmenu_controller (Utilities|Casting|CastToBP_RTSMenuController NewPlayer))
      (Utilities|Array|Add (Variables|Default|GetAll_ConnectedPlayers) _asbp_rtsmenu_controller)
      (Default|CreateLobbyMenu _asbp_rtsmenu_controller)
      (Default|InitialSetup _asbp_rtsmenu_controller))))

(fn ConstructionScript)