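; Player controller for the RTS menu and multiplayer lobby, handling UI-only input, lobby and loading screens, and leaving sessions.
; ROS_ events forward join, ready, team, faction, color and map changes to functions that store them on BP_RTS_PlayerState.
; These functions loop over the GameState PlayerArray, calling ROC events on player states to update lobby views.
; A readiness check enables the host's Start Game button once enough players are all ready.
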(event Custom|EndClientSession
  ;[1 1 1] End Session
  (|DestroySession self
    (:then
      (Game|OpenLevel(byObjectReference) "/Game/UI/UI_Maps/Mainmenu.Mainmenu"))))

(event Custom|CreateLoadScreen
  ;[1 1 1] Show loadscreen
  (CallFunction|UIShowLoadScreen))

(event Custom|ROS_SwitchFaction
  (params (InPlayerState :type Player%20State%20Object%20Reference) (InPlayerName :type Text) (InFactionName :type String))
  (CallFunction|SwitchFaction InPlayerState InPlayerName InFactionName))

(event Custom|ROS_SwitchColor
  (params (InPlayerState :type Player%20State%20Object%20Reference) (InPlayerName :type Text) (InColor :type Name))
  (CallFunction|SwitchColor InPlayerState InPlayerName InColor))

(event Custom|ROS_CheckPlayerReadyness
  ;[1 1 1] Check if player is ready and update widget accordingly
  (if (> (Utilities|Array|Length (Variables|/Script/Engine.GameStateBase|GetPlayerArray (Game|GetGameState))) (Variables|Default|GetNumOfPlayerToStart))
    (for _array_element (Variables|/Script/Engine.GameStateBase|GetPlayerArray (Game|GetGameState))
      ;;[0 0 0] Check if Everyplayer has clicked Ready
      (bind _asbp_rts_player_state (Utilities|Casting|CastToBP_RTS_PlayerState _array_element))
      (if (not (Variables|/Game/Framework/Gameplay/BP_RTS_PlayerState.BP_RTS_PlayerState_C|GetIsReady _asbp_rts_player_state))
        (Variables|Default|SetEveryoneIsReady false)))
    (bind _asbp_game_instance (Utilities|Casting|CastToBP_GameInstance (Game|GetGameInstance)))
    (if (Variables|Default|GetEveryoneIsReady)
      (Networking|SwitchHasAuthority
        (:Authority
          ;;[0 0 0] Allows Host to start game
          (Rendering|Components|TextRender|SetText (Variables|/Game/UI/UI_Blueprints/UI_Lobby/WB_LobbyMenuUI.WB_LobbyMenuUI_C|GetText_StartGamebtn (Variables|/Game/Framework/BP_GameInstance.BP_GameInstance_C|GetWB_LobbyMenu _asbp_game_instance)) "Start Game")
          (Widget|SetIsEnabled (Variables|/Game/UI/UI_Blueprints/UI_Lobby/WB_LobbyMenuUI.WB_LobbyMenuUI_C|GetStartGame_btn (Variables|/Game/Framework/BP_GameInstance.BP_GameInstance_C|GetWB_LobbyMenu _asbp_game_instance)) true)))
      (else
        ;;[0 0 0] Updates button and text when all players are not ready
        (Variables|Default|SetEveryoneIsReady true)
        (Networking|SwitchHasAuthority
          (:Authority
            (Rendering|Components|TextRender|SetText (Variables|/Game/UI/UI_Blueprints/UI_Lobby/WB_LobbyMenuUI.WB_LobbyMenuUI_C|GetText_StartGamebtn (Variables|/Game/Framework/BP_GameInstance.BP_GameInstance_C|GetWB_LobbyMenu _asbp_game_instance)) (Variables|/Game/UI/UI_Blueprints/UI_Lobby/WB_LobbyMenuUI.WB_LobbyMenuUI_C|GetText_StartGameVariablebtn (Variables|/Game/Framework/BP_GameInstance.BP_GameInstance_C|GetWB_LobbyMenu _asbp_game_instance)))
            (Widget|SetIsEnabled (Variables|/Game/UI/UI_Blueprints/UI_Lobby/WB_LobbyMenuUI.WB_LobbyMenuUI_C|GetStartGame_btn (Variables|/Game/Framework/BP_GameInstance.BP_GameInstance_C|GetWB_LobbyMenu _asbp_game_instance)) false)))))))

(event Custom|ROS_SwitchMap
  (params (InPlayerState :type Player%20State%20Object%20Reference) (InSelectedMap :type Name))
  (CallFunction|SwitchMap InPlayerState InSelectedMap))

(event Custom|Initial_Setup
  ;[1 1 1] Update when player joins
)

(event Custom|ROS_BeginPlayLobby
  (params (InPlayerState :type Player%20State%20Object%20Reference) (InPlayerName :type Text))
  (CallFunction|BeginPlayLobby InPlayerState InPlayerName))

(event Custom|ROC_UpdateLevelSelection
  (params (LevelRowName :type Name))
  (bind _wb_lobbymenu (Variables|Default|GetWB_LobbyMenu))
  ;[1 1 1] Update Lobby Selected Map
  (Utilities|IsValid _wb_lobbymenu
    (:Is%20Valid
      (Default|UpdateLevelSelection _wb_lobbymenu LevelRowName))))

(event Custom|ROS_SwitchTeam
  (params (InPlayerState :type Player%20State%20Object%20Reference) (InPlayerTeam :type Name) (InPlayerName :type Text))
  (CallFunction|SwitchTeam InPlayerState InPlayerTeam InPlayerName))

(event Custom|ROS_NewPlayerJoined
  (params (InPlayerState :type Player%20State%20Object%20Reference))
  (CallFunction|NewPlayerJoined InPlayerState))

(event Custom|ROS_PlayerReady
  (params (InPlayerState :type Player%20State%20Object%20Reference) (InPlayerName :type Text) (InIsReady :type Boolean))
  (CallFunction|PlayerReady InPlayerState InPlayerName InIsReady))

(event EventBeginPlay
  ;[1 1 1] Fix mouse on screen
  (if (Pawn|IsLocalController)
    (Variables|Default|SetbShowMouseCursor true)
    (Input|SetInputModeUIOnly self 0 "DoNotLock" false)))

(fn ConstructionScript)

(fn UIShowLobbyMenu
  (Utilities|IsValid (Variables|Default|GetWB_LobbyMenu)
    (:Is%20Valid
      _)
    (:Is%20Not%20Valid
      (bind _returnvalue (UserInterface|CreateWidget "/Game/UI/UI_Blueprints/UI_Lobby/WB_LobbyMenuUI.WB_LobbyMenuUI_C" self))
      (bind _output_get (Variables|Default|SetWB_LobbyMenu _returnvalue))))
  (UserInterface|Viewport|AddtoViewport (Variables|Default|GetWB_LobbyMenu) 0)
  (return _output_get))

(fn LoadSavedProfile
  (bind _returnvalue (SaveGame|DoesSaveGameExist (LocalVariables|GetLcl_SlotName)))
  (if _returnvalue
    _
    (else
      (bind _returnvalue_2 (SaveGame|CreateSaveGameObject "/Game/SaveData/SG_PlayerProfile.SG_PlayerProfile_C"))
      (SaveGame|SaveGametoSlot _returnvalue_2 (LocalVariables|GetLcl_SlotName))))
  (bind _returnvalue_3 (SaveGame|LoadGamefromSlot (LocalVariables|GetLcl_SlotName)))
  (bind _assg_player_profile (Utilities|Casting|CastToSG_PlayerProfile _returnvalue_3))
  (Variables|Default|SetPlayerProfileInfo (Variables|/Game/SaveData/SG_PlayerProfile.SG_PlayerProfile_C|GetPlayerProfile _assg_player_profile))
  (return))

(fn UIShowLoadScreen
  (Viewport|RemoveAllWidgets)
  (Utilities|IsValid (Variables|Default|GetWB_LoadScreen)
    (:Is%20Valid
      _)
    (:Is%20Not%20Valid
      (bind _returnvalue (UserInterface|CreateWidget "/Game/UI/UI_Blueprints/WB_LoadScreen.WB_LoadScreen_C" self))
      (Variables|Default|SetWB_LoadScreen _returnvalue)))
  (UserInterface|Viewport|AddtoViewport (Variables|Default|GetWB_LoadScreen) 0)
  (return))

(fn BeginPlayLobby
  (params (InPlayerState :type Player%20State%20Object%20Reference) (InPlayerName :type Text))
  (bind _asbp_rts_player_state (Utilities|Casting|CastToBP_RTS_PlayerState InPlayerState))
  (Variables|/Game/Framework/Gameplay/BP_RTS_PlayerState.BP_RTS_PlayerState_C|SetMyPlayerName _asbp_rts_player_state InPlayerName)
  (for _array_element (Variables|/Script/Engine.GameStateBase|GetPlayerArray (Game|GetGameState)) ; Iterate through the playerlist
    (bind _asbp_rts_player_state_2 (Utilities|Casting|CastToBP_RTS_PlayerState _array_element))
    (Default|ROCAddPlayer _asbp_rts_player_state (Variables|/Game/Framework/Gameplay/BP_RTS_PlayerState.BP_RTS_PlayerState_C|GetMyPlayerName _asbp_rts_player_state_2) (Variables|/Game/Framework/Gameplay/BP_RTS_PlayerState.BP_RTS_PlayerState_C|GetMyFactionName _asbp_rts_player_state_2) (Variables|/Game/Framework/Gameplay/BP_RTS_PlayerState.BP_RTS_PlayerState_C|GetMyTeamName _asbp_rts_player_state_2) (Variables|/Game/Framework/Gameplay/BP_RTS_PlayerState.BP_RTS_PlayerState_C|GetMyColor _asbp_rts_player_state_2) (Variables|/Game/Framework/Gameplay/BP_RTS_PlayerState.BP_RTS_PlayerState_C|GetIsReady _asbp_rts_player_state_2))))

(fn SwitchTeam
  (params (InPlayerState :type Player%20State%20Object%20Reference) (InPlayerTeam :type Name) (InPlayerName :type Text))
  (bind _asbp_rts_player_state (Utilities|Casting|CastToBP_RTS_PlayerState InPlayerState))
  (Variables|/Game/Framework/Gameplay/BP_RTS_PlayerState.BP_RTS_PlayerState_C|SetMyTeamName _asbp_rts_player_state InPlayerTeam)
  (for _array_element (Variables|/Script/Engine.GameStateBase|GetPlayerArray (Game|GetGameState))
    (bind _asbp_rts_player_state_2 (Utilities|Casting|CastToBP_RTS_PlayerState _array_element))
    (Default|ROCSwitchTeam _asbp_rts_player_state_2 (== _asbp_rts_player_state_2 InPlayerState) InPlayerTeam InPlayerName)))

(fn NewPlayerJoined
  (params (InPlayerState :type Player%20State%20Object%20Reference))
  (for _array_element (Variables|/Script/Engine.GameStateBase|GetPlayerArray (Game|GetGameState))
    (bind _asbp_rts_player_state (Utilities|Casting|CastToBP_RTS_PlayerState _array_element))
    (if (not (== _asbp_rts_player_state InPlayerState))
      (bind _asbp_rts_player_state_2 (Utilities|Casting|CastToBP_RTS_PlayerState InPlayerState))
      (Default|ROCAddPlayer _asbp_rts_player_state (Variables|/Game/Framework/Gameplay/BP_RTS_PlayerState.BP_RTS_PlayerState_C|GetMyPlayerName _asbp_rts_player_state_2) "" "None" "None" false))))

(fn PlayerReady
  (params (InPlayerState :type Player%20State%20Object%20Reference) (InPlayerName :type Text) (InIsReady :type Boolean))
  ;[1 1 1] When ready, we tell the server that i am ready, please update for the other clients
  (bind _asbp_rts_player_state (Utilities|Casting|CastToBP_RTS_PlayerState InPlayerState))
  (Variables|/Game/Framework/Gameplay/BP_RTS_PlayerState.BP_RTS_PlayerState_C|SetIsReady _asbp_rts_player_state InIsReady)
  (for _array_element (Variables|/Script/Engine.GameStateBase|GetPlayerArray (Game|GetGameState))
    ;;[1 1 1] Tell other clients to find their representation of me and update it
    (bind _asbp_rts_player_state_2 (Utilities|Casting|CastToBP_RTS_PlayerState _array_element))
    (Default|ROCPlayerReady _asbp_rts_player_state_2 InPlayerName InIsReady)))

(fn SwitchFaction
  (params (InPlayerState :type Player%20State%20Object%20Reference) (InPlayerName :type Text) (InFactionName :type String))
  (bind _asbp_rts_player_state (Utilities|Casting|CastToBP_RTS_PlayerState InPlayerState))
  (Variables|/Game/Framework/Gameplay/BP_RTS_PlayerState.BP_RTS_PlayerState_C|SetMyFactionName _asbp_rts_player_state InFactionName)
  (for _array_element (Variables|/Script/Engine.GameStateBase|GetPlayerArray (Game|GetGameState))
    (bind _asbp_rts_player_state_2 (Utilities|Casting|CastToBP_RTS_PlayerState _array_element))
    (Default|ROCSwitchFaction _asbp_rts_player_state_2 (== _asbp_rts_player_state_2 InPlayerState) InPlayerName InFactionName)))

(fn SwitchColor
  (params (InPlayerState :type Player%20State%20Object%20Reference) (InPlayerName :type Text) (InColor :type Name))
  (bind _asbp_rts_player_state (Utilities|Casting|CastToBP_RTS_PlayerState InPlayerState))
  (Variables|/Game/Framework/Gameplay/BP_RTS_PlayerState.BP_RTS_PlayerState_C|SetMyColor _asbp_rts_player_state InColor)
  (for _array_element (Variables|/Script/Engine.GameStateBase|GetPlayerArray (Game|GetGameState))
    (bind _asbp_rts_player_state_2 (Utilities|Casting|CastToBP_RTS_PlayerState _array_element))
    (Default|ROCSwitchColor _asbp_rts_player_state_2 (== _asbp_rts_player_state_2 InPlayerState) InPlayerName InColor)))

(fn SwitchMap
  (params (InPlayerState :type Player%20State%20Object%20Reference) (InSelectedMap :type Name))
  (bind _asbp_rts_player_state (Utilities|Casting|CastToBP_RTS_PlayerState InPlayerState))
  (Variables|/Game/Framework/Gameplay/BP_RTS_PlayerState.BP_RTS_PlayerState_C|SetMapName _asbp_rts_player_state InSelectedMap)
  (for _array_element (Variables|/Script/Engine.GameStateBase|GetPlayerArray (Game|GetGameState))
    ;[1 1 1] Tell other clients to find their map image and update it
    (bind _asbp_rts_player_state_2 (Utilities|Casting|CastToBP_RTS_PlayerState _array_element))
    (Default|ROCSwitchMap _asbp_rts_player_state_2 InSelectedMap)))