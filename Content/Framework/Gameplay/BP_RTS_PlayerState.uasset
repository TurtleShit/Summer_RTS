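; RTS player state that relays lobby changes (player add/remove, faction, team, color, ready, map) to BP_GameInstance.
; ROC_ events wrap matching functions that cast to the game instance and call its function of the same name.
; Faction, team and color switches also store the value on the game instance first when the player is local.
; CopyProperties carries SPlayerProfile to the new player state during seamless server travel.
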(event Custom|ROC_AddPlayer
  (params (InPlayerName :type Text) (InFactionName :type String) (InTeamName :type Name) (InColor :type Name) (InIsReady :type Boolean))
  (CallFunction|AddPlayer InPlayerName InFactionName InTeamName InColor InIsReady))

(event Custom|ROC_SwitchTeam
  (params (InIsPlayerLocal :type Boolean) (InTeamName :type Name) (InPlayerName :type Text))
  (CallFunction|SwitchTeam InIsPlayerLocal InTeamName InPlayerName))

(event Custom|ROC_PlayerReady
  (params (InPlayerName :type Text) (InIsReady :type Boolean))
  (CallFunction|PlayerReady InPlayerName InIsReady))

(event Custom|ROC_SwitchFaction
  (params (InIsPlayerLocal :type Boolean) (InPlayerName :type Text) (InFactionName :type String))
  (CallFunction|SwitchFaction InIsPlayerLocal InPlayerName InFactionName))

(event Custom|ROC_SwitchColor
  (params (IsPlayerLocal :type Boolean) (InPlayerName :type Text) (InColor :type Name))
  (CallFunction|SwitchColor IsPlayerLocal InPlayerName InColor))

(event Custom|ROC_SwitchMap
  (params (InMapName :type Name))
  (CallFunction|SwitchMap InMapName))

(event Custom|ROC_RemovePlayer
  (params (InPlayerToBeRemoved :type Text))
  (CallFunction|RemovePlayer InPlayerToBeRemoved))

(event EventCopyProperties
  (params (NewPlayerState :type Player%20State%20Object%20Reference))
  ;[1 1 1] PlayerProfile remains consistent. ONLY when using semlesstravel
  (bind _asbp_rts_player_state (Utilities|Casting|CastToBP_RTS_PlayerState NewPlayerState))
  (Variables|BP_RTS_PlayerState_C|SetS_PlayerProfile _asbp_rts_player_state (Variables|Default|GetS_PlayerProfile)))

(fn ConstructionScript)

(fn AddPlayer
  (params (InPlayerName :type Text) (InFactionName :type String) (InTeamName :type Name) (InColor :type Name) (InIsReady :type Boolean))
  (bind _asbp_game_instance (Utilities|Casting|CastToBP_GameInstance (Game|GetGameInstance)))
  (Default|AddPlayer _asbp_game_instance InPlayerName InFactionName InTeamName InColor InIsReady))

(fn SwitchTeam
  (params (InIsPlayerLocal :type Boolean) (InTeamName :type Name) (InPlayerName :type Text))
  (if InIsPlayerLocal
    ;[1 1 1] Assign value locally
    (bind _asbp_game_instance (Utilities|Casting|CastToBP_GameInstance (Game|GetGameInstance)))
    (Variables|/Game/Framework/BP_GameInstance.BP_GameInstance_C|SetTeamName _asbp_game_instance InTeamName))
  ;[1 1 1] Tell server to update Team change to all clients
  (bind _asbp_game_instance_2 (Utilities|Casting|CastToBP_GameInstance (Game|GetGameInstance)))
  (Default|SwitchTeam _asbp_game_instance_2 InTeamName InPlayerName))

(fn PlayerReady
  (params (InPlayerName :type Text) (InIsReady :type Boolean))
  (bind _asbp_game_instance (Utilities|Casting|CastToBP_GameInstance (Game|GetGameInstance)))
  (Default|PlayerReady _asbp_game_instance InPlayerName InIsReady))

(fn SwitchFaction
  (params (InIsPlayerLocal :type Boolean) (InPlayerName :type Text) (InFactionName :type String))
  (if InIsPlayerLocal
    ;[1 1 1] Assign value locally
    (bind _asbp_game_instance (Utilities|Casting|CastToBP_GameInstance (Game|GetGameInstance)))
    (Variables|/Game/Framework/BP_GameInstance.BP_GameInstance_C|SetFactionName _asbp_game_instance (Utilities|String|StringToName InFactionName)))
  ;[1 1 1] Tell server to update faction change to all clients
  (bind _asbp_game_instance_2 (Utilities|Casting|CastToBP_GameInstance (Game|GetGameInstance)))
  (Default|SwitchFaction _asbp_game_instance_2 InPlayerName InFactionName))

(fn SwitchColor
  (params (IsPlayerLocal :type Boolean) (InPlayerName :type Text) (InColor :type Name))
  (if IsPlayerLocal
    (bind _asbp_game_instance (Utilities|Casting|CastToBP_GameInstance (Game|GetGameInstance)))
    (Variables|/Game/Framework/BP_GameInstance.BP_GameInstance_C|SetColorName _asbp_game_instance InColor))
  ;[1 1 1] Tell server to update Team change to all clients
  (bind _asbp_game_instance_2 (Utilities|Casting|CastToBP_GameInstance (Game|GetGameInstance)))
  (Default|SwitchColor _asbp_game_instance_2 InColor InPlayerName))

(fn SwitchMap
  (params (InMapName :type Name))
  (bind _asbp_game_instance (Utilities|Casting|CastToBP_GameInstance (Game|GetGameInstance)))
  (Default|SwitchMap _asbp_game_instance InMapName))

(fn RemovePlayer
  (params (InPlayerToBeRemoved :type Text))
  (bind _asbp_game_instance (Utilities|Casting|CastToBP_GameInstance (Game|GetGameInstance)))
  (Default|RemovePlayer _asbp_game_instance InPlayerToBeRemoved))